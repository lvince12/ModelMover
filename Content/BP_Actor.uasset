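; Actor that drives a skeletal mesh through a Control Rig component, procedurally moving its hand and head controls at runtime.
; On rig pre-initialization, it maps the complete skeletal mesh as the rig's output.
; Each Tick reads the left hand, right hand and head control transforms in rig space and writes them back offset along +Y, keeping rotation and scale.
; The offset is added per frame without delta-time scaling.
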(event `self.ControlRig.OnPreInitializeDelegate`
  (params (Component :type "ControlRigComponent Object Reference"))
  (`ControlRigComponent.AddMappedCompleteSkeletalMesh` Component (`self.SkeletalMesh`) "Output"))

(event `self.ReceiveTick`
  (params (DeltaSeconds :type "Float (single-precision)"))
  (bind (_returnvalue_location _returnvalue_rotation _returnvalue_scale) (`KismetMathLibrary.BreakTransform` (`ControlRigComponent.GetControlTransform` (`self.ControlRig`) "hand_l_ctrl" "RigSpace")))
  (bind (_returnvalue_location_2 _returnvalue_rotation_2 _returnvalue_scale_2) (`KismetMathLibrary.BreakTransform` (`ControlRigComponent.GetControlTransform` (`self.ControlRig`) "hand_r_ctrl" "RigSpace")))
  (bind (_returnvalue_location_3 _returnvalue_rotation_3 _returnvalue_scale_3) (`KismetMathLibrary.BreakTransform` (`ControlRigComponent.GetControlTransform` (`self.ControlRig`) "head_ctrl" "RigSpace")))
  (`ControlRigComponent.SetControlTransform` (`self.ControlRig`) "hand_l_ctrl" (`KismetMathLibrary.MakeTransform` (+ _returnvalue_location (0.0 5.0 0.0)) _returnvalue_rotation _returnvalue_scale) "RigSpace")
  (`ControlRigComponent.SetControlTransform` (`self.ControlRig`) "hand_r_ctrl" (`KismetMathLibrary.MakeTransform` (+ _returnvalue_location_2 (0.0 5.0 0.0)) _returnvalue_rotation_2 _returnvalue_scale_2) "RigSpace")
  (`ControlRigComponent.SetControlTransform` (`self.ControlRig`) "head_ctrl" (`KismetMathLibrary.MakeTransform` (+ _returnvalue_location_3 (0.0 5.0 0.0)) _returnvalue_rotation_3 _returnvalue_scale_3) "RigSpace"))

(fn `UserConstructionScript`)